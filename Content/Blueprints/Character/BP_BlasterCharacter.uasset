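; BP_BlasterCharacter is the player character Blueprint, handling melee hits, elimination, enemy targeting cleanup, sniper scope UI and game end.
; Hand attacks sphere-trace between arm and hand sockets, damaging BP_Enemy or BP_EnemyBoss.
; It registers with BP_BlasterGameMode; ServerElimmed calls MultiElimmed to ragdoll, unregisters and decrements revive count.
; ResetEnemyTarget releases tracked enemies and bosses, while EndGame shows the return menu and pauses.
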(event Custom|ServerElimmed
  (CallFunction|MultiElimmed)
  (bind _asbp_blaster_game_mode (Utilities|Casting|CastToBP_BlasterGameMode (Game|GetGameMode)))
  (Utilities|Array|RemoveItem (Variables|/Game/Blueprints/GameModes/BP_BlasterGameMode.BP_BlasterGameMode_C|GetPlayers _asbp_blaster_game_mode) self)
  (Default|ChangePlayersTeamMsg _asbp_blaster_game_mode)
  (Variables|/Game/Blueprints/GameModes/BP_BlasterGameMode.BP_BlasterGameMode_C|SetPlayerReviveTimes _asbp_blaster_game_mode (- (Variables|/Game/Blueprints/GameModes/BP_BlasterGameMode.BP_BlasterGameMode_C|GetPlayerReviveTimes _asbp_blaster_game_mode) 1)))

(event Custom|MultiElimmed
  (bind _mesh (Variables|Character|GetMesh))
  (Physics|SetSimulatePhysics _mesh true)
  (Collision|SetCollisionEnabled _mesh "QueryAndPhysics"))

(event Custom|RightHandAttack
  (bind _mesh (Variables|Character|GetMesh))
  (Variables|Default|SetStartTraceLocation (Transformation|GetSocketLocation _mesh "ArmR"))
  (Variables|Default|SetEndTraceLocation (Transformation|GetSocketLocation _mesh "HandR"))
  (CallFunction|AttackTrace))

(event Custom|LeftHandAttack
  (bind _mesh (Variables|Character|GetMesh))
  (Variables|Default|SetStartTraceLocation (Transformation|GetSocketLocation _mesh "ArmL"))
  (Variables|Default|SetEndTraceLocation (Transformation|GetSocketLocation _mesh "HandL"))
  (CallFunction|AttackTrace))

(event Custom|ChangeTeamMsg
  (params (Overlay :type WBP%20Character%20Overlay%20Object%20Reference))
  (Default|InitialPlayersHPBar Overlay))

(event Custom|AttackTrace
  (bind _outhit (Collision|SphereTraceForObjects (Variables|Default|GetStartTraceLocation) (Variables|Default|GetEndTraceLocation) 1e+01 (Variables|Default|GetTraceObjects) false 0 "None"))
  (Utilities|Casting|CastToBP_Enemy (.HitActor (Collision|BreakHitResult _outhit))
    (:then
      _)
    (:CastFailed
      (Utilities|Casting|CastToBP_EnemyBoss (.HitActor (Collision|BreakHitResult _outhit)))))
  (Game|Damage|ApplyDamage (.HitActor (Collision|BreakHitResult _outhit)) 15.0 (Pawn|GetController) 0)
  (Audio|PlaySoundatLocation "/Game/Assets/Sounds/Foley/Jab_Cue.Jab_Cue" (Transformation|GetActorLocation) "0, 0, 0" 1.0 1.0 0.0 0 0 0))

(event Custom|EndGame
  (params (EndResult :type Text))
  (Variables|Default|SetEndResult EndResult)
  (bind _asbp_blaster_player_controller (Utilities|Casting|CastToBP_BlasterPlayerController (Pawn|GetController)))
  (Class|BlasterPlayerController|ShowReturntoMainMenu _asbp_blaster_player_controller)
  (Game|SetGamePaused true))

(event EventBeginPlay
  (bind _asbp_blaster_game_mode (Utilities|Casting|CastToBP_BlasterGameMode (Game|GetGameMode)))
  (Utilities|Array|Add (Variables|/Game/Blueprints/GameModes/BP_BlasterGameMode.BP_BlasterGameMode_C|GetPlayers _asbp_blaster_game_mode) self))

(event EventResetEnemyTarget
  (Utilities|FlowControl|Sequence
    (:then_0
      (for _array_element (Variables|Default|GetEnemyAimSelf)
        (Utilities|IsValid _array_element
          (:Is%20Valid
            (Default|ResetTarget _array_element))))
      (Utilities|Array|Clear (Variables|Default|GetEnemyAimSelf)))
    (:then_1
      (for _array_element_2 (Variables|Default|GetBossAimSelf)
        (Utilities|IsValid _array_element_2
          (:Is%20Valid
            (Variables|/Game/Blueprints/Enemy/Boss/BP_EnemyBoss.BP_EnemyBoss_C|SetOldTarget _array_element_2 (Variables|/Game/Blueprints/Enemy/Boss/BP_EnemyBoss.BP_EnemyBoss_C|GetTargetCharacter _array_element_2))
            (Variables|/Game/Blueprints/Enemy/Boss/BP_EnemyBoss.BP_EnemyBoss_C|SetTargetCharacter _array_element_2 0)
            (Default|ChangeTarget _array_element_2))))
      (Utilities|Array|Clear (Variables|Default|GetBossAimSelf)))))

(event EventShowSniperScopeWidget
  (params (bShowScope :type Boolean))
  (Utilities|IsValid (Variables|Default|GetSniperScopeWidget)
    (:Is%20Valid
      _)
    (:Is%20Not%20Valid
      (bind _returnvalue (UserInterface|CreateWidget "/Game/Blueprints/HUD/WBP_SniperScope.WBP_SniperScope_C"))
      (bind _output_get (Variables|Default|SetSniperScopeWidget _returnvalue))
      (UserInterface|Viewport|AddtoViewport _output_get 0)))
  (if bShowScope
    (Utilities|IsValid (Variables|Default|GetSniperScopeWidget)
      (:Is%20Valid
        (UserInterface|Animation|PlayAnimation (Variables|Default|GetSniperScopeWidget) (Variables|/Game/Blueprints/HUD/WBP_SniperScope.WBP_SniperScope_C|GetScopeZoomIn (Variables|Default|GetSniperScopeWidget)) 0.0 1 "Forward" 1.0 false)
        (Audio|PlaySound2D "/Game/Assets/MilitaryWeapSilver/Sound/SniperRifle/Cues/SniperRifle_ZoomIn_Cue.SniperRifle_ZoomIn_Cue" 1.0 1.0 0.0 0 0)))
    (else
      (Utilities|IsValid (Variables|Default|GetSniperScopeWidget)
        (:Is%20Valid
          (UserInterface|Animation|PlayAnimation (Variables|Default|GetSniperScopeWidget) (Variables|/Game/Blueprints/HUD/WBP_SniperScope.WBP_SniperScope_C|GetScopeZoomIn (Variables|Default|GetSniperScopeWidget)) 0.0 1 "Reverse" 3.0 false)
          (Audio|PlaySound2D "/Game/Assets/MilitaryWeapSilver/Sound/SniperRifle/Cues/SniperRifle_ZoomOut_Cue.SniperRifle_ZoomOut_Cue" 1.0 1.0 0.0 0 0))))))

(fn ConstructionScript)