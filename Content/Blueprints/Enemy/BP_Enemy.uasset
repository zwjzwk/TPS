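; Melee enemy that hunts the first BP_NPC found until damage switches its target to the attacking controller, unless already targeting a BlasterCharacter.
; Tick drives AIMoveTo, range checks and smooth facing, alternating two attack montages on cooldown.
; A separate Attack event rechecks range before applying damage.
; Hits slow it; death removes it from the game mode, awards score, ragdolls it and may spawn a random drop.
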(event Custom|GetNPCTarget
  (bind _outactors (Actor|GetAllActorsOfClass "/Game/Blueprints/NPC/BP_NPC.BP_NPC_C"))
  (Variables|Default|SetTargetCharacterController (Pawn|GetController (Utilities|Array|Get(acopy) _outactors))))

(event Custom|MultiPlayHitMontage
  (Animation|Montage|PlayMontage (Variables|Character|GetMesh) (Variables|Default|GetGetHitMontage)
    (:OnCompleted
      (Variables|/Script/Engine.CharacterMovementComponent|SetMaxWalkSpeed (Variables|Character|GetCharacterMovement) 4.5e+02))))

(event Custom|MultiEnemyDeath
  (bind _hpbar (Variables|Default|GetHPBar))
  (Variables|Default|SetDeath true)
  (Utilities|IsValid _hpbar
    (:Is%20Valid
      (Components|DestroyComponent _hpbar))
    (:Is%20Not%20Valid
      _))
  (Collision|SetCollisionEnabled (Variables|Character|GetMesh) "NoCollision")
  (Components|Animation|PlayAnimation (Variables|Character|GetMesh) "/Game/Assets/ThirdPerson/Mannequin/Animations/EnemyDeath.EnemyDeath" false)
  (Utilities|FlowControl|Delay 0.9)
  (Physics|SetSimulatePhysics (Variables|Character|GetMesh) true)
  (Collision|SetCollisionEnabled (Variables|Character|GetMesh) "PhysicsOnly")
  (Utilities|FlowControl|Delay 2.0)
  (Actor|DestroyActor))

(event Custom|Attack
  (bind _targetcharactercontroller (Variables|Default|GetTargetCharacterController))
  (bind _returnvalue (Pawn|GetControlledPawn _targetcharactercontroller))
  (Utilities|IsValid _targetcharactercontroller
    (:Is%20Valid
      (if (<= (Math|Vector|Distance(Vector) (Transformation|GetActorLocation _returnvalue) (Transformation|GetActorLocation)) (Variables|Default|GetAttackRange))
        (Game|Damage|ApplyDamage _returnvalue (Variables|Default|GetAttackDamage) (Pawn|GetController) self)))))

(event Custom|IsInAttackRange
  (CallFunction|MultiPlayJabMontage))

(event Custom|MultiPlayJabMontage
  (Variables|Default|SetCanAttack false)
  (Variables|/Script/Engine.CharacterMovementComponent|SetMaxWalkSpeed (Variables|Character|GetCharacterMovement) 0.0)
  (Utilities|FlowControl|FlipFlop
    (:A
      (Animation|Montage|PlayMontage (Variables|Character|GetMesh) (Variables|Default|GetAttackAMontage)
        (:then
          (Utilities|FlowControl|Delay (Variables|Default|GetAttackCD) :!label _label)
          (Variables|Default|SetCanAttack true))
        (:OnCompleted
          (Variables|/Script/Engine.CharacterMovementComponent|SetMaxWalkSpeed (Variables|Character|GetCharacterMovement) 4.5e+02 :!label _label_2))))
    (:B
      (Animation|Montage|PlayMontage (Variables|Character|GetMesh) (Variables|Default|GetAttackBMontage)
        (:then
          (goto _label))
        (:OnCompleted
          (goto _label_2))))))

(event Custom|IsInRange
  (bind _targetcharactercontroller (Variables|Default|GetTargetCharacterController))
  (if (!= _targetcharactercontroller 0)
    (if (and (<= (Math|Vector|Distance(Vector) (Transformation|GetActorLocation (Pawn|GetControlledPawn _targetcharactercontroller)) (Transformation|GetActorLocation)) (Variables|Default|GetAttackRange)) (Variables|Default|GetCanAttack))
      (CallFunction|IsinAttackRange))))

(event Custom|FaceToCharacter
  (bind _capsulecomponent (Variables|Default|GetCapsuleComponent))
  (bind _asbp_blaster_character (Utilities|Casting|CastToBP_BlasterCharacter (Pawn|GetControlledPawn (Variables|Default|GetTargetCharacterController))))
  (Transformation|SetWorldRotation (Variables|Default|GetCapsuleComponent) (Math|Interpolation|RInterpTo (Transformation|GetWorldRotation _capsulecomponent) (Math|Rotator|FindLookatRotation (Transformation|GetWorldLocation _capsulecomponent) (Transformation|GetWorldLocation (Variables|/Script/Engine.Character|GetCapsuleComponent _asbp_blaster_character))) (Variables|Default|GetDelta%20Seconds) 2.0) false false))

(event Custom|ResetTarget
  (CallFunction|GetNPCTarget)
  (bind _asbp_npc (Utilities|Casting|CastToBP_NPC (Pawn|GetControlledPawn (Variables|Default|GetTargetCharacterController))))
  (Transformation|SetActorRotation (Math|Rotator|FindLookatRotation (Transformation|GetWorldLocation (Variables|Default|GetCapsuleComponent)) (Transformation|GetWorldLocation (Variables|/Script/Engine.Character|GetCapsuleComponent _asbp_npc)))))

(event EventBeginPlay
  (bind _aswbp_enemy_hpbar (Utilities|Casting|CastToWBP_EnemyHPBar (UserInterface|GetUserWidgetObject (Variables|Default|GetHPBar))))
  (Variables|/Game/Blueprints/HUD/WBP_EnemyHPBar.WBP_EnemyHPBar_C|SetEnemy _aswbp_enemy_hpbar self))

(event Game|Damage|EventAnyDamage
  (params (Damage :type Float%20%28single-precision%29) (DamageType :type Damage%20Type%20Object%20Reference) (InstigatedBy :type Controller%20Object%20Reference) (DamageCauser :type Actor%20Object%20Reference))
  (CallFunction|MultiPlayHitMontage)
  (Variables|/Script/Engine.CharacterMovementComponent|SetMaxWalkSpeed (Variables|Character|GetCharacterMovement) 5e+01)
  (Utilities|Casting|CastToBlasterCharacter (Pawn|GetControlledPawn (Variables|Default|GetTargetCharacterController))
    (:then
      _)
    (:CastFailed
      (bind _output_get (Variables|Default|SetTargetCharacterController InstigatedBy))
      (bind _asbp_blaster_character (Utilities|Casting|CastToBP_BlasterCharacter (Pawn|GetControlledPawn _output_get))
        (:then
          (Utilities|Array|Add (Variables|/Game/Blueprints/Character/BP_BlasterCharacter.BP_BlasterCharacter_C|GetEnemyAimSelf _asbp_blaster_character) self))
        (:CastFailed
          _))))
  (bind _output_get_2 (Variables|Default|SetHP_Current (Math|Float|Truncate (Math|Float|Clamp(Float) (- (Math|Conversions|ToFloat(Integer) (Variables|Default|GetHP_Current)) Damage) 0.0 (Math|Conversions|ToFloat(Integer) (Variables|Default|GetHP_Max))))))
  (if (<= _output_get_2 0)
    (if (not (Variables|Default|GetDeath))
      (CallFunction|MultiEnemyDeath)
      (bind _asbp_blaster_game_mode (Utilities|Casting|CastToBP_BlasterGameMode (Game|GetGameMode)))
      (Utilities|Array|RemoveItem (Variables|/Game/Blueprints/GameModes/BP_BlasterGameMode.BP_BlasterGameMode_C|GetEnemys _asbp_blaster_game_mode) self)
      (bind _asbp_blaster_player_state (Utilities|Casting|CastToBP_BlasterPlayerState (Variables|/Script/Engine.Controller|GetPlayerState InstigatedBy)))
      (Class|BlasterPlayerState|AddtoScore _asbp_blaster_player_state 1.0)
      (if (== (Math|Random|RandomIntegerinRange 0 (Variables|Default|GetDropRange)) 0)
        (Utilities|FlowControl|Delay 2.2)
        (Game|SpawnActorfromClass (Utilities|Array|Get(acopy) (Variables|Default|GetDrop) (Math|Random|RandomIntegerinRange 0 23)) (Math|Transform|MakeTransform (Transformation|GetSocketLocation (Variables|Character|GetMesh) "pelvis") "0, 0, 0" "1,1,1") "Undefined" 0 0)))))

(event EventTick
  (params (DeltaSeconds :type Float%20%28single-precision%29))
  (bind _targetcharactercontroller (Variables|Default|GetTargetCharacterController))
  (Variables|Default|SetDelta%20Seconds DeltaSeconds)
  (Utilities|IsValid _targetcharactercontroller
    (:Is%20Valid
      (AI|AIMoveTo self "0, 0, 0" _targetcharactercontroller (Variables|Default|GetMoveAcceptRadius) true
        (:then
          (CallFunction|IsinRange)
          (CallFunction|FacetoCharacter))))
    (:Is%20Not%20Valid
      (CallFunction|GetNPCTarget))))

(fn ConstructionScript)