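; Wizard enemy Blueprint that adds a magic projectile attack.
; The MagicAttack event spawns a BP_MagicBall at the location passed in as LeftOrRight.
; The ball takes the mesh's world rotation with a 90-degree yaw offset, compensating for mesh orientation.
; BeginPlay and Tick are unused, and the construction script only calls the parent.
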(event Custom|MagicAttack
  (params (LeftOrRight :type Vector))
  (bind _mesh (Variables|Character|GetMesh))
  (bind _returnvalue (Transformation|GetWorldRotation _mesh))
  ;[1 1 1] 魔法攻击
  (Game|SpawnActorfromClass "/Game/Blueprints/Enemy/BP_MagicBall.BP_MagicBall_C" (Math|Transform|MakeTransform LeftOrRight (Math|Rotator|MakeRotator (.roll _returnvalue) (.pitch _returnvalue) (+ (.yaw _returnvalue) 9e+01)) "1,1,1") "Undefined" 0 0))

(event EventBeginPlay
  (|CallParentFunction) ; This node is disabled and will not be called.\nDrag off pins to build functionality.
)

(event EventTick
  (params (DeltaSeconds :type Float%20%28single-precision%29))
  (|CallParentFunction DeltaSeconds) ; This node is disabled and will not be called.\nDrag off pins to build functionality.
)

(fn ConstructionScript
  (|CallParentFunction))