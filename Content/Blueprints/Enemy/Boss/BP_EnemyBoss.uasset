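; Samurai boss enemy that hunts BP_BlasterCharacter players, feeding target, strafe and combat readiness to the AC_EnemyBoss blackboard.
; Random timers trigger defense, strafing and lunging special attacks, while montage attacks deal damage through sphere traces.
; Incoming hits can be blocked or dodged; at half health it changes material, hits harder and pulses poison damage.
; Death ragdolls the body, awards score and spawns a drop.
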(event Custom|Attack
  (if (not (Variables|Default|GetAttackMontage))
    (Variables|Default|SetAttackMontage true)
    (if (== (Math|Random|RandomIntegerinRange 0 7) 0)
      (Variables|Default|SetDodgeMontagePlay true)
      (CallFunction|ServerPlayMontage "/Game/Assets/GhostSamurai_Katana/GhostSamurai_Katana/Animation/Apose/Dodge/Root/GhostSamurai_APose_Dodge_B_Root_Montage.GhostSamurai_APose_Dodge_B_Root_Montage")
      (else
        (CallFunction|ServerPlayMontage (Utilities|Array|Get(acopy) (Variables|Default|GetAttack%20Montage%20to%20Play) (Math|Random|RandomIntegerinRange 0 4)))))))

(event Custom|ServerPlayMontage
  (params (Montage :type Anim%20Montage%20Object%20Reference))
  (CallFunction|MulticastPlayMontage Montage))

(event Custom|ChangeColor
  (Rendering|Material|SetMaterial (Variables|Character|GetMesh) 0 "/Game/Assets/Materials/MI_BossPart2.MI_BossPart2")
  (Rendering|SetVisibility (Variables|Default|GetSkill) true false)
  (Variables|Default|SetAttackDamage 5e+01)
  (Variables|Default|SetSpecialAttackDamage 1e+02)
  (Utilities|Time|SetTimerbyEvent (delegate Custom|PoisonAttack) 1.0 true))

(event Custom|SpecialAttackSphere
  (bind _arrow1 (Variables|Default|GetArrow1))
  (bind _returnvalue (Transformation|GetWorldLocation _arrow1))
  (bind (_outhit _returnvalue_2) (Collision|SphereTraceForObjects _returnvalue (+ _returnvalue (* (Math|Vector|GetForwardVector _arrow1) 1.8e+02)) 8e+01 (Variables|Default|GetTraceTypes) false 0 "None"))
  (if _returnvalue_2
    (Utilities|Casting|CastToBP_BlasterCharacter (.HitActor (Collision|BreakHitResult _outhit)))
    (Game|Damage|ApplyDamage (.HitActor (Collision|BreakHitResult _outhit)) (Variables|Default|GetSpecialAttackDamage) (Pawn|GetController) 0)
    (Audio|PlaySound2D "/Game/Assets/Sounds/Sword/SwordHit_Cue.SwordHit_Cue" 1.0 1.0 0.0 0 0)))

(event Custom|ReadyToFight
  (bind _asac_enemy_boss (Utilities|Casting|CastToAC_EnemyBoss (AI|GetAIController self)))
  (AI|Components|Blackboard|SetValueasBool (AI|GetBlackboard _asac_enemy_boss) (Utilities|Name|MakeLiteralName "ReadyToFight") true)
  (Variables|Default|SetEquipMontagePlay false)
  (Variables|Default|SetHitMontagePlay false))

(event Custom|ChangeTarget
  (bind _outactors (Actor|GetAllActorsOfClass "/Game/Blueprints/Character/BP_BlasterCharacter.BP_BlasterCharacter_C"))
  (for _array_element _outactors
    (if (!= _array_element (Variables|Default|GetOldTarget))
      (bind _output_get (Variables|Default|SetTargetCharacter _array_element))
      (Utilities|Array|Add (Variables|/Game/Blueprints/Character/BP_BlasterCharacter.BP_BlasterCharacter_C|GetBossAimSelf _output_get) self)
      (bind _asac_enemy_boss (Utilities|Casting|CastToAC_EnemyBoss (AI|GetAIController self)))
      (Variables|Default|SetOldTarget 0)
      (AI|Components|Blackboard|SetValueasObject (AI|GetBlackboard _asac_enemy_boss) (Utilities|Name|MakeLiteralName "Target") (Variables|Default|GetTargetCharacter))))
  (if (== (Variables|Default|GetTargetCharacter) 0)
    (Utilities|FlowControl|Delay 5.0)
    (CallFunction|ChangeTarget)))

(event Custom|Run
  (bind _runvalue (Timeline|RunTimeLine Play)
    (:Update
      (Variables|/Script/Engine.CharacterMovementComponent|SetMaxWalkSpeed (Variables|Character|GetCharacterMovement) _runvalue))))

(event Custom|ResetAttack
  (Variables|Default|SetAttackMontage false)
  (Variables|Default|SetDodgeMontagePlay false)
  (Variables|Default|SetDefense false)
  (bind _output_get (Variables|Default|SetStrafe false))
  (bind _asac_enemy_boss (Utilities|Casting|CastToAC_EnemyBoss (AI|GetAIController self)))
  (AI|Components|Blackboard|SetValueasBool (AI|GetBlackboard _asac_enemy_boss) (Utilities|Name|MakeLiteralName "Strafe") _output_get))

(event Custom|PoisonAttack
  (bind _returnvalue (Transformation|GetActorLocation))
  (bind (_outhit _returnvalue_2) (Collision|SphereTraceForObjects _returnvalue _returnvalue 7e+02 (Variables|Default|GetTraceTypes) false 0 "None"))
  (if _returnvalue_2
    (bind _asbp_blaster_character (Utilities|Casting|CastToBP_BlasterCharacter (.HitActor (Collision|BreakHitResult _outhit))))
    (Game|Damage|ApplyDamage _asbp_blaster_character (Variables|Default|GetPoisonDamage) (Pawn|GetController) 0)))

(event Custom|StopRunning
  (bind _runvalue (Timeline|RunTimeLine Reverse)
    (:Update
      (Variables|/Script/Engine.CharacterMovementComponent|SetMaxWalkSpeed (Variables|Character|GetCharacterMovement) _runvalue))))

(event Custom|SetDefense
  (if (Math|Boolean|ANDBoolean (Variables|Default|GetEquip) (not (Variables|Default|GetPlayingDeathMontage)) (not (Variables|Default|GetAttackMontage)))
    (CallFunction|StopRunning)
    (Variables|Default|SetDefense true)
    (Utilities|FlowControl|Delay (Math|Random|RandomFloatinRange 5.0 1e+01))
    (Variables|Default|SetDefense false)))

(event Custom|SetStrafe
  (if (Math|Boolean|ANDBoolean (Variables|Default|GetEquip) (not (Variables|Default|GetPlayingDeathMontage)) (not (Variables|Default|GetAttackMontage)))
    (bind _output_get (Variables|Default|SetStrafe true))
    (bind _asac_enemy_boss (Utilities|Casting|CastToAC_EnemyBoss (AI|GetAIController self)))
    (AI|Components|Blackboard|SetValueasBool (AI|GetBlackboard _asac_enemy_boss) (Utilities|Name|MakeLiteralName "Strafe") _output_get)))

(event Custom|MulticastPlayMontage
  (params (Montage :type Anim%20Montage%20Object%20Reference))
  (Animation|Montage|PlayMontage (Variables|Character|GetMesh) Montage))

(event Custom|MultiDeath
  (Utilities|FlowControl|Delay 0.9)
  (Physics|SetSimulatePhysics (Variables|Character|GetMesh) true)
  (Collision|SetCollisionEnabled (Variables|Character|GetMesh) "PhysicsOnly")
  (Utilities|FlowControl|Delay 3.0)
  (Actor|DestroyActor))

(event Custom|SpecialAttack
  (bind _returnvalue (Transformation|GetActorForwardVector))
  (bind _targetcharacter (Variables|Default|GetTargetCharacter))
  (bind _targetcharacter_2 (Variables|Default|GetTargetCharacter))
  (bind _targetcharacter_3 (Variables|Default|GetTargetCharacter))
  (bind _returnvalue_2 (Transformation|GetActorLocation _targetcharacter_3))
  (bind _returnvalue_3 (Transformation|GetActorLocation _targetcharacter))
  (bind _returnvalue_4 (Transformation|GetActorLocation _targetcharacter_2))
  (if (Math|Boolean|ANDBoolean (Variables|Default|GetEquip) (not (Variables|Default|GetPlayingDeathMontage)) (not (Variables|Default|GetAttackMontage)))
    (Variables|Default|SetAttackMontage true)
    (if (Math|Random|RandomBool)
      (CallFunction|ServerPlayMontage "/Game/Assets/GhostSamurai_Katana/GhostSamurai_Katana/Animation/Apose/Attack/Root/GhostSamurai_APose_JumpAttack02_Root_Montage.GhostSamurai_APose_JumpAttack02_Root_Montage")
      (Character|LaunchCharacter (Math|Vector|MakeVector (.x _returnvalue) (.y _returnvalue) 7e+02) true true)
      (Utilities|FlowControl|Delay 0.2)
      (Utilities|IsValid (Variables|Default|GetTargetCharacter)
        (:Is%20Valid
          (Variables|Default|SetTargetLocation (Math|Vector|MakeVector (+ (.x _returnvalue_4) 2e+02) (.y _returnvalue_4) (+ (.z _returnvalue_4) 2e+01)))
          (Utilities|FlowControl|Sequence
            (:then_0
              (bind _value (Timeline|Timeline_1 PlayFromStart)
                (:Update
                  (Transformation|SetActorLocation (Math|Vector|Lerp(Vector) (Transformation|GetActorLocation) (Variables|Default|GetTargetLocation) _value) false false))))
            (:then_1
              (Utilities|FlowControl|Delay 0.2)
              (Variables|Default|SetTargetLocation (Math|Vector|MakeVector (+ (.x _returnvalue_2) 2e+02) (.y _returnvalue_2) (+ (.z _returnvalue_2) 2e+01)))))))
      (else
        (CallFunction|ServerPlayMontage "/Game/Assets/GhostSamurai_Katana/GhostSamurai_Katana/Animation/Apose/Attack/Root/GhostSamurai_APose_SPAttack01_Root_Montage.GhostSamurai_APose_SPAttack01_Root_Montage")
        (Utilities|FlowControl|Delay 0.9)
        (Variables|Default|SetTargetLocation (Math|Vector|MakeVector (+ (.x _returnvalue_3) 2e+02) (.y _returnvalue_3) (.z (Transformation|GetActorLocation))))
        (bind _value_2 (Timeline|Timeline_0 PlayFromStart)
          (:Update
            (Transformation|SetActorLocation (Math|Vector|Lerp(Vector) (Transformation|GetActorLocation) (Variables|Default|GetTargetLocation) _value_2) false false)))))))

(event Custom|ReadyCombat
  (Variables|Default|SetEquip true)
  (Utilities|FlowControl|DoOnce false
    (:Completed
      (Variables|Default|SetEquipMontagePlay true)
      (CallFunction|ServerPlayMontage "/Game/Assets/GhostSamurai_Katana/GhostSamurai_Katana/Animation/Common/Root/GhostSamurai_APose_Equip02_Root_Montage.GhostSamurai_APose_Equip02_Root_Montage"))))

(event Custom|AttackSphere
  (bind _arrow1 (Variables|Default|GetArrow1))
  (bind _returnvalue (Transformation|GetWorldLocation _arrow1))
  (bind (_outhit _returnvalue_2) (Collision|SphereTraceForObjects _returnvalue (+ _returnvalue (* (Math|Vector|GetForwardVector _arrow1) 1.5e+02)) 8e+01 (Variables|Default|GetTraceTypes) false 0 "None"))
  (if _returnvalue_2
    (bind _asbp_blaster_character (Utilities|Casting|CastToBP_BlasterCharacter (.HitActor (Collision|BreakHitResult _outhit))))
    (Game|Damage|ApplyDamage _asbp_blaster_character (Variables|Default|GetAttackDamage) (Pawn|GetController) 0)
    (Audio|PlaySound2D "/Game/Assets/Sounds/Sword/SwordHit_Cue.SwordHit_Cue" 1.0 1.0 0.0 0 0)))

(event EventBeginPlay
  (Utilities|FlowControl|Sequence
    (:then_0
      (bind _aswbp_boss_hpbar (Utilities|Casting|CastToWBP_BossHPBar (UserInterface|GetUserWidgetObject (Variables|Default|GetHPBar))))
      (Variables|/Game/Blueprints/HUD/WBP_BossHPBar.WBP_BossHPBar_C|SetBoss _aswbp_boss_hpbar self))
    (:then_1
      (bind _outactors (Actor|GetAllActorsOfClass "/Game/Blueprints/Character/BP_BlasterCharacter.BP_BlasterCharacter_C"))
      (bind _output_get (Variables|Default|SetTargetCharacter (Utilities|Array|Get(acopy) _outactors)))
      (bind _asac_enemy_boss (Utilities|Casting|CastToAC_EnemyBoss (AI|GetAIController self)))
      (AI|Components|Blackboard|SetValueasObject (AI|GetBlackboard _asac_enemy_boss) (Utilities|Name|MakeLiteralName "Target") _output_get))
    (:then_2
      (Utilities|Array|Add (Variables|/Game/Blueprints/Character/BP_BlasterCharacter.BP_BlasterCharacter_C|GetBossAimSelf (Variables|Default|GetTargetCharacter)) self))
    (:then_3
      (Utilities|Time|SetTimerbyEvent (delegate Custom|SetDefense) (Math|Random|RandomFloatinRange 2e+01 3e+01) true))
    (:then_4
      (Utilities|Time|SetTimerbyEvent (delegate Custom|SetStrafe) (Math|Random|RandomFloatinRange 15.0 3e+01) true))
    (:then_5
      (Utilities|Time|SetTimerbyEvent (delegate Custom|SpecialAttack) (Math|Random|RandomFloatinRange 1e+01 18.0) true))
    (:then_6
      (Transformation|SetAbsolute (Variables|Default|GetSkill) false true false))))

(event EventTick
  (params (DeltaSeconds :type Float%20%28single-precision%29))
  (Utilities|IsValid (Variables|Default|GetTargetCharacter)
    (:Is%20Valid
      (Transformation|SetActorRotation (Math|Interpolation|RInterpTo (Transformation|GetActorRotation) (Math|Rotator|FindLookatRotation (Transformation|GetActorLocation) (Transformation|GetActorLocation (Variables|Default|GetTargetCharacter))) (Utilities|Time|GetWorldDeltaSeconds) 25.0))
      (Pawn|Input|AddMovementInput (Transformation|GetActorRightVector) (Variables|Default|GetStrafe%20Value) false))))

(event Game|Damage|EventAnyDamage
  (params (Damage :type Float%20%28single-precision%29) (DamageType :type Damage%20Type%20Object%20Reference) (InstigatedBy :type Controller%20Object%20Reference) (DamageCauser :type Actor%20Object%20Reference))
  (bind _hpbar (Variables|Default|GetHPBar))
  (Variables|Default|SetAttackMontage false)
  (if (not (Math|Boolean|ORBoolean (Variables|Default|GetDodgeMontagePlay) (Variables|Default|GetPlayingDeathMontage) (Variables|Default|GetEquipMontagePlay)))
    (Variables|Default|SetHitMontagePlay true)
    (if (Variables|Default|GetDefense)
      (CallFunction|ServerPlayMontage "/Game/Assets/GhostSamurai_Katana/GhostSamurai_Katana/Animation/Defense/Root/GhostSamurai_DefenseR_Hit01_Root_Montage.GhostSamurai_DefenseR_Hit01_Root_Montage")
      (Utilities|FlowControl|Delay 0.3)
      (Variables|Default|SetHitMontagePlay false)
      (elif (and (== (Math|Random|RandomIntegerinRange 0 8) 0) (Variables|Default|GetFirstGetHit))
        (Variables|Default|SetDodgeMontagePlay true)
        (CallFunction|ServerPlayMontage (Utilities|Array|Get(acopy) (Variables|Default|GetDodgeMontages) (Math|Random|RandomIntegerinRange 0 3)))
        (Utilities|FlowControl|Delay 0.3)
        (Variables|Default|SetHitMontagePlay false)
        (else
          (Variables|Default|SetFirstGetHit true)
          (if (<= Damage 5e+01)
            _
            (else
              (CallFunction|ServerPlayMontage "/Game/Assets/GhostSamurai_Katana/GhostSamurai_Katana/Animation/Apose/Hit/Root/GhostSamurai_APose_Hit_F_Root_Montage.GhostSamurai_APose_Hit_F_Root_Montage")))
          (bind _output_get (Variables|Default|SetCurrentHP (Math|Integer|Clamp(Integer) (- (Variables|Default|GetCurrentHP) (Math|Float|Truncate Damage)) 0 (Variables|Default|GetMaxHP))))
          (if (<= _output_get 0)
            (Utilities|IsValid _hpbar
              (:Is%20Valid
                (Components|DestroyComponent _hpbar)
                (CallFunction|ServerPlayMontage "/Game/Assets/GhostSamurai_Katana/GhostSamurai_Katana/Animation/Apose/Die/Root/GhostSamurai_APose_Die01_Root_Montage.GhostSamurai_APose_Die01_Root_Montage")
                (Variables|Default|SetPlayingDeathMontage true)
                (Pawn|UnPossess (AI|GetAIController self))
                (CallFunction|MultiDeath)
                (bind _asbp_blaster_game_mode (Utilities|Casting|CastToBP_BlasterGameMode (Game|GetGameMode)))
                (Utilities|Array|RemoveItem (Variables|/Game/Blueprints/GameModes/BP_BlasterGameMode.BP_BlasterGameMode_C|GetEnemys _asbp_blaster_game_mode) self)
                (bind _asbp_blaster_player_state (Utilities|Casting|CastToBP_BlasterPlayerState (Variables|/Script/Engine.Controller|GetPlayerState InstigatedBy)))
                (Class|BlasterPlayerState|AddtoScore _asbp_blaster_player_state 1.0)
                (Utilities|FlowControl|Delay 2.0)
                (Game|SpawnActorfromClass (Variables|Default|GetDrop) (Math|Transform|MakeTransform (Transformation|GetSocketLocation (Variables|Character|GetMesh) "pelvis") "0, 0, 0" "1,1,1") "Undefined" 0 0)))
            (else
              (bind _asac_enemy_boss (Utilities|Casting|CastToAC_EnemyBoss (AI|GetAIController self)))
              (AI|Components|Blackboard|SetValueasObject (AI|GetBlackboard _asac_enemy_boss) (Utilities|Name|MakeLiteralName "Target") (Variables|Default|GetTargetCharacter))
              (if (<= (Variables|Default|GetCurrentHP) (/ (Variables|Default|GetMaxHP) 2))
                (CallFunction|ChangeColor)))))))))

(fn ConstructionScript)

(fn CalculateLastInput
  (bind _charactermovement (Variables|Character|GetCharacterMovement))
  (bind _returnvalue (Pawn|Components|PawnMovement|GetLastInputVector _charactermovement))
  (bind _output_get (Variables|Default|SetInput? (Class|KismetMathLibrary|NotEqualExactlyVectorVector _returnvalue "0, 0, 0")))
  (Variables|Default|SetLastInput _returnvalue)
  (if _output_get
    (Variables|Default|SetLastRotation (Math|Rotator|MakeRotfromX _returnvalue))))

(fn RInterptoRotation
  (params (IsInterp? :type Boolean))
  (if IsInterp?
    (Transformation|SetActorRotation (Math|Interpolation|RInterpTo (Transformation|GetActorRotation) (Variables|Default|GetLastRotation) (Utilities|Time|GetWorldDeltaSeconds) 2e+01))))