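; Game mode for Blaster that runs a scripted sequence of enemy waves and decides when the match is won or lost.
; After a start delay, Tick advances a non-looping MultiGate, via a Delay, whenever Enemys empties or the wave timer expires.
; Waves spawn regular, wizard and boss enemies at BP_EnemySpawnPoint actors, ending with a tougher boss, then victory.
; Tick also ends the game for all characters once PlayerReviveTimes drops below zero.
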(event Custom|SpawnEnemy1
  (for _array_element (Variables|Default|GetEnemyPoints)
    (bind _returnvalue (Game|SpawnActorfromClass "/Game/Blueprints/Enemy/BP_Enemy.BP_Enemy_C" (Math|Transform|MakeTransform (Transformation|GetActorLocation _array_element) "0, 0, 0" "1,1,1") "Undefined" 0 0))
    (Utilities|Array|Add (Variables|Default|GetEnemys) _returnvalue)))

(event Custom|SpawnEnemy3
  (for (_array_element _array_index) (Variables|Default|GetEnemyPoints)
    (if (>= _array_index 4)
      (bind _returnvalue (Game|SpawnActorfromClass "/Game/Blueprints/Enemy/BP_Enemy.BP_Enemy_C" (Math|Transform|MakeTransform (Transformation|GetActorLocation _array_element) "0, 0, 0" "1,1,1") "Undefined" 0 0))
      (Utilities|Array|Add (Variables|Default|GetEnemys) _returnvalue)
      (else
        (bind _returnvalue_2 (Game|SpawnActorfromClass "/Game/Blueprints/Enemy/BP_Enemy_Wizard.BP_Enemy_Wizard_C" (Math|Transform|MakeTransform (Transformation|GetActorLocation _array_element) "0, 0, 0" "1,1,1") "Undefined" 0 0))
        (Utilities|Array|Add (Variables|Default|GetEnemys) _returnvalue_2)))))

(event Custom|SpawnBoss
  (params (Second :type Boolean))
  (bind _returnvalue (Game|SpawnActorfromClass "/Game/Blueprints/Enemy/Boss/BP_EnemyBoss.BP_EnemyBoss_C" (Math|Transform|MakeTransform (Transformation|GetActorLocation (Utilities|Array|Get(acopy) (Variables|Default|GetEnemyPoints) 4)) "0, 0, 0" "1,1,1") "Undefined" 0 0))
  (if Second
    (Variables|/Game/Blueprints/Enemy/Boss/BP_EnemyBoss.BP_EnemyBoss_C|SetCurrentHP _returnvalue 2000)
    (Variables|/Game/Blueprints/Enemy/Boss/BP_EnemyBoss.BP_EnemyBoss_C|SetMaxHP _returnvalue 2000))
  (Utilities|Array|Add (Variables|Default|GetEnemys) _returnvalue))

(event Custom|ChangePlayersTeamMsg
  (for _array_element (Variables|Default|GetPlayers)
    (Variables|/Game/Blueprints/Character/BP_BlasterCharacter.BP_BlasterCharacter_C|SetShouldChangeTeamMsg _array_element true)))

(event Custom|EndGame
  (params (EndResult :type Text))
  (for _array_element (Variables|Default|GetPlayers)
    (Default|EndGame _array_element EndResult)))

(event Custom|SpawnEnemy2
  (for (_array_element _array_index) (Variables|Default|GetEnemyPoints)
    (if (<= _array_index 6)
      (bind _returnvalue (Game|SpawnActorfromClass "/Game/Blueprints/Enemy/BP_Enemy.BP_Enemy_C" (Math|Transform|MakeTransform (Transformation|GetActorLocation _array_element) "0, 0, 0" "1,1,1") "Undefined" 0 0))
      (Utilities|Array|Add (Variables|Default|GetEnemys) _returnvalue)
      (else
        (bind _returnvalue_2 (Game|SpawnActorfromClass "/Game/Blueprints/Enemy/BP_Enemy_Wizard.BP_Enemy_Wizard_C" (Math|Transform|MakeTransform (Transformation|GetActorLocation _array_element) "0, 0, 0" "1,1,1") "Undefined" 0 0))
        (Utilities|Array|Add (Variables|Default|GetEnemys) _returnvalue_2)))))

(event EventBeginPlay
  (bind _outactors (Actor|GetAllActorsOfClass "/Game/Blueprints/Enemy/BP_EnemySpawnPoint.BP_EnemySpawnPoint_C"))
  (Variables|Default|SetEnemyPoints _outactors)
  (Utilities|FlowControl|Delay 11.0)
  (Actor|Tick|SetActorTickEnabled true))

(event EventTick
  (params (DeltaSeconds :type Float%20%28single-precision%29))
  (Variables|Default|SetCurrentUpdateTime (- (Variables|Default|GetCurrentUpdateTime) DeltaSeconds))
  (Utilities|FlowControl|Sequence
    (:then_0
      (if (or (== (Utilities|Array|Length (Variables|Default|GetEnemys)) 0) (<= (Variables|Default|GetCurrentUpdateTime) 0.0))
        (Utilities|FlowControl|Delay 5.0)
        (Utilities|FlowControl|MultiGate false false -1
          (:Out%200
            (CallFunction|SpawnEnemy1)
            (Variables|Default|SetCurrentUpdateTime (Variables|Default|GetEnemyUpdateTime) :!label _label))
          (:Out%201
            (CallFunction|SpawnEnemy2)
            (goto _label))
          (:Out%202
            (CallFunction|SpawnEnemy3)
            (goto _label))
          (:Out%203
            (CallFunction|SpawnBoss false)
            (goto _label))
          (:Out%204
            (CallFunction|SpawnEnemy1)
            (goto _label))
          (:Out%205
            (CallFunction|SpawnEnemy3)
            (goto _label))
          (:Out%206
            (CallFunction|SpawnBoss true)
            (Variables|Default|SetCurrentUpdateTime 9999.0))
          (:Out%207
            (CallFunction|EndGame "消灭了全部敌人，获得胜利！")
            (Actor|Tick|SetActorTickEnabled false)))))
    (:then_1
      (if (< (Variables|Default|GetPlayerReviveTimes) 0)
        (bind _outactors (Actor|GetAllActorsOfClass "/Game/Blueprints/Character/BP_BlasterCharacter.BP_BlasterCharacter_C"))
        (for _array_element _outactors
          (Default|EndGame _array_element "复活次数已用尽！"))
        (Actor|Tick|SetActorTickEnabled false)))))

(fn ConstructionScript)