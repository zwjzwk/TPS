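; BP_NPC is the protected NPC in a Blaster game mode, whose death fails the match.
; On BeginPlay it hands itself to its WBP_NPCHPBar widget so the bar can reference it.
; AnyDamage lowers current HP clamped between zero and max, and at zero a DoOnce calls EndGame on BP_BlasterGameMode with a failed-protection message and stops that game mode's tick.
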(event EventBeginPlay
  (bind _aswbp_npchpbar (Utilities|Casting|CastToWBP_NPCHPBar (UserInterface|GetUserWidgetObject (Variables|Default|GetHPBar))))
  (Variables|/Game/Blueprints/HUD/WBP_NPCHPBar.WBP_NPCHPBar_C|SetNPC _aswbp_npchpbar self))

(event Game|Damage|EventAnyDamage
  (params (Damage :type Float%20%28single-precision%29) (DamageType :type Damage%20Type%20Object%20Reference) (InstigatedBy :type Controller%20Object%20Reference) (DamageCauser :type Actor%20Object%20Reference))
  (bind _output_get (Variables|Default|SetHP_Current (Math|Float|Truncate (Math|Float|Clamp(Float) (- (Math|Conversions|ToFloat(Integer) (Variables|Default|GetHP_Current)) Damage) 0.0 (Math|Conversions|ToFloat(Integer) (Variables|Default|GetHP_Max))))))
  (if (<= _output_get 0)
    (Utilities|FlowControl|DoOnce false
      (:Completed
        (bind _asbp_blaster_game_mode (Utilities|Casting|CastToBP_BlasterGameMode (Game|GetGameMode)))
        (Default|EndGame _asbp_blaster_game_mode "未能成功守护NPC！")
        (Actor|Tick|SetActorTickEnabled _asbp_blaster_game_mode)))))

(fn ConstructionScript)